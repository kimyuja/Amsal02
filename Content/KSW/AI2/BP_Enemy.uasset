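; BP_Enemy is an AI enemy character with a modular body, controlled by BP_EnemyCon.
; On BeginPlay, its shoes, pants, hand and torso meshes follow the main mesh's pose through leader pose components.
; Each tick it reads the controller's Warning flag and, while set, halts movement immediately, calls UpdateStack to update a warning stack and prints debug values.
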(event `self.ReceiveBeginPlay`
  (`SkinnedMeshComponent.SetLeaderPoseComponent` (`self.Shoes`) (`self.Mesh`) false false)
  (`SkinnedMeshComponent.SetLeaderPoseComponent` (`self.Pants`) (`self.Mesh`) false false)
  (`SkinnedMeshComponent.SetLeaderPoseComponent` (`self.Hand`) (`self.Mesh`) false false)
  (`SkinnedMeshComponent.SetLeaderPoseComponent` (`self.Torso`) (`self.Mesh`) false false))

(event `self.ReceiveTick`
  (params (DeltaSeconds :type "Float (single-precision)"))
  (bind _asbp_enemy_con (cast `/Game/KSW/AI2/BP_EnemyCon` (`self.GetController`)))
  (bind _bwarning (`/Game/KSW/AI2/BP_EnemyCon.bWarning` _asbp_enemy_con))
  (if _bwarning
    (`KismetSystemLibrary.PrintString` (`KismetStringLibrary.Conv_BoolToString` _bwarning))
    (`MovementComponent.StopMovementImmediately` (`self.CharacterMovement`))
    (`self.UpdateStack` 1)
    (`KismetSystemLibrary.PrintString` (`KismetStringLibrary.Conv_IntToString` (`self.warningstack`)))))

(fn `UserConstructionScript`)