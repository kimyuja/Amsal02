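; BP_HitManAI is an enemy AI character with a warning state and a stealth neck-assassination death.
; Each Tick it reads BP_EnemyCon, raising the warning stack and SeeWeapon on Warning, and adding a far larger amount on SeeDeath.
; SneakNeckAssasin plays the dying montage, disables collision, triggers delayed ragdoll and returns the AssasinREF transform.
; A PlantDeath_targetLoc event moves the actor to a hard-coded location.
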(event `self.ReceiveBeginPlay`)

(event `self.ReceiveTick`
  (params (DeltaSeconds :type "Float (single-precision)"))
  (bind _asbp_enemy_con (cast `/Game/KSW/AI2/BP_EnemyCon` (`self.GetController`)))
  (`|ExecutionSequence`
    (:`then_0`
      (if (`/Game/KSW/AI2/BP_EnemyCon.bWarning` _asbp_enemy_con)
        (set `self.bSeeWeapon` true)
        (`self.UpdateWarningStack` 5)
        (else
          (set `self.bSeeWeapon` false))))
    (:`then_1`
      (if (`EnemyCon.bSeeDeath` _asbp_enemy_con)
        (`self.UpdateWarningStack` 2000)))))

(event `PlantDeath_targetLoc`
  (`self.K2_SetActorLocation` (-110.0 -596.0 56.0)))

(event `Ragdoll`
  (`KismetSystemLibrary.Delay` 1.2)
  (`PrimitiveComponent.SetSimulatePhysics` (`self.Mesh`) true))

(fn `Sneak Neck Assasin`
  (returns (`REF Location` :type "Vector Structure") (`Assasin Rotation` :type "Rotator Structure"))
  (bind _assasin_ref (`self.Assasin REF`))
  (`self.PlayAnimMontage` "/Game/KSW/Anime/UnFixed/Dying_Backwards_Montage.Dying_Backwards_Montage")
  (`self.Ragdoll`)
  (set `self.bIsDie` true)
  (`SceneComponent.SetVisibility` (`self.warningComp`) false false)
  (`PrimitiveComponent.SetCollisionEnabled` (`self.CapsuleComponent`) "NoCollision")
  (`PrimitiveComponent.SetCollisionEnabled` (`self.headShot`) "NoCollision")
  (`PrimitiveComponent.SetNotifyRigidBodyCollision` (`self.Mesh`) false)
  (return (`SceneComponent.K2_GetComponentLocation` _assasin_ref) (`SceneComponent.K2_GetComponentRotation` _assasin_ref)))

(fn `UserConstructionScript`)