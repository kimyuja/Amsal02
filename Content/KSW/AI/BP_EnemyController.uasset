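; BP_EnemyController is an enemy AI controller that runs BT_Enemy on possess and tracks player detection through AI Perception.
; Each successful sensing update of a Player-tagged actor cancels the forget timer and increments a warning counter, mirrored to the Blackboard.
; At the warning threshold it sets line of sight and the target actor.
; Any other perception update starts a timer that clears both and resets the warning.
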(event `self.ReceiveBeginPlay`)

(event `self.ReceivePossess`
  (params (PossessedPawn :type "Pawn Object Reference"))
  (`self.RunBehaviorTree` "/Game/KSW/AI/BT_Enemy.BT_Enemy"))

(event `self.AIPerception.OnTargetPerceptionUpdated`
  (params (Actor :type "Actor Object Reference") (Stimulus :type "AIStimulus Structure"))
  (bind _blackboard (`self.Blackboard`))
  (if (and (`self.ActorHasTag` Actor "Player") (`.bSuccessfullySensed` (break `AIStimulus` Stimulus)))
    (`KismetSystemLibrary.K2_ClearAndInvalidateTimerHandle` (`self.enemyTimer`))
    (bind _result (`/Engine/EditorBlueprintResources/StandardMacros.IncrementFloat` (`self.warning para`))
      (:`  `
        (bind _output_get (set `self.warning para` _result))
        (if (>= _output_get 5.0)
          (`BlackboardComponent.SetValueAsBool` _blackboard (`self.hasLineOfSight`) true)
          (`BlackboardComponent.SetValueAsObject` _blackboard (`self.enemyActor`) Actor))
        (`BlackboardComponent.SetValueAsFloat` _blackboard (`self.warning`) (`self.warning para`))))
    (else
      (bind _returnvalue (`KismetSystemLibrary.K2_SetTimerDelegate` (delegate `StartEnemyTimer`) (`self.lineOfSightTimer`)))
      (set `self.enemyTimer` _returnvalue))))

(event `StartEnemyTimer`
  (bind _blackboard (`self.Blackboard`))
  (`BlackboardComponent.SetValueAsBool` _blackboard (`self.hasLineOfSight`) false)
  (`BlackboardComponent.SetValueAsObject` _blackboard (`self.enemyActor`) null)
  (bind _output_get (set `self.warning para` 0.0))
  (`BlackboardComponent.SetValueAsFloat` _blackboard (`self.warning`) _output_get))

(fn `UserConstructionScript`)