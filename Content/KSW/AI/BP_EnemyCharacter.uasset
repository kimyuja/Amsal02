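; Enemy AI character with modular body meshes following the main mesh pose, a life value and a warning text display.
; Damage lowers Life, and at zero the character stops moving, turns ragdoll and hides the warning.
; Tick refreshes the warning while WarningPara is mid-range on the first BP_EnemyController found in the level, not necessarily its own.
; Pistol bullet headshot and body-hit damage logic exists but is disconnected from the overlap events.
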(event `self.ReceiveBeginPlay`
  (`SkinnedMeshComponent.SetLeaderPoseComponent` (`self.Shoes`) (`self.Mesh`) false false)
  (`SkinnedMeshComponent.SetLeaderPoseComponent` (`self.Pants`) (`self.Mesh`) false false)
  (`SkinnedMeshComponent.SetLeaderPoseComponent` (`self.Hand`) (`self.Mesh`) false false)
  (`SkinnedMeshComponent.SetLeaderPoseComponent` (`self.Torso`) (`self.Mesh`) false false)
  (bind _outactors (`GameplayStatics.GetAllActorsOfClass` "/Game/KSW/AI/BP_EnemyController.BP_EnemyController_C"))
  (bind _asbp_enemy_controller (cast `/Game/KSW/AI/BP_EnemyController` (`|GetArrayItem` _outactors)))
  (set `self.As BP Enemy Controller` _asbp_enemy_controller))

(event `self.ReceiveAnyDamage`
  (params (Damage :type "Float (single-precision)") (DamageType :type "DamageType Object Reference") (InstigatedBy :type "Controller Object Reference") (DamageCauser :type "Actor Object Reference"))
  (bind _mesh (`self.Mesh`))
  (bind _output_get (set `self.Life` (`KismetMathLibrary.FClamp` (- (`self.Life`) Damage) 0.0 100.0)))
  (`KismetSystemLibrary.PrintString` (`KismetStringLibrary.Conv_DoubleToString` _output_get))
  (if (<= (`self.Life`) 0.0)
    (`CharacterMovementComponent.DisableMovement` (`self.CharacterMovement`))
    (`PrimitiveComponent.SetCollisionEnabled` _mesh "QueryAndPhysics")
    (`PrimitiveComponent.SetCollisionEnabled` (`self.Torso`) "QueryAndPhysics")
    (`PrimitiveComponent.SetCollisionEnabled` (`self.Shoes`) "QueryAndPhysics")
    (`PrimitiveComponent.SetCollisionEnabled` (`self.Pants`) "QueryAndPhysics")
    (`PrimitiveComponent.SetCollisionEnabled` (`self.Hand`) "QueryAndPhysics")
    (`PrimitiveComponent.SetCollisionEnabled` (`self.Headshot`) "QueryAndPhysics")
    (`SkeletalMeshComponent.SetAllBodiesSimulatePhysics` _mesh true)
    (`SkeletalMeshComponent.SetAllBodiesSimulatePhysics` (`self.Torso`) true)
    (`SkeletalMeshComponent.SetAllBodiesSimulatePhysics` (`self.Shoes`) true)
    (`SkeletalMeshComponent.SetAllBodiesSimulatePhysics` (`self.Pants`) true)
    (`SkeletalMeshComponent.SetAllBodiesSimulatePhysics` (`self.Hand`) true)
    (`SkeletalMeshComponent.SetAllBodiesPhysicsBlendWeight` _mesh 1.0 false)
    (`PrimitiveComponent.SetCollisionEnabled` (`self.CapsuleComponent`) "NoCollision")
    (`PrimitiveComponent.SetCollisionEnabled` (`self.Headshot`) "NoCollision")
    (`SceneComponent.SetVisibility` (`self.Warning`) false false)))

(event `self.ReceiveTick`
  (params (DeltaSeconds :type "Float (single-precision)"))
  (bind _warning_para (`/Game/KSW/AI/BP_EnemyController.warning para` (`self.As BP Enemy Controller`)))
  (if (<= _warning_para 4.9)
    (if (>= _warning_para 0.1)
      (`self.UpdateWarning` (`self.Warning Text`)))))

(event `self.CapsuleComponent.OnComponentBeginOverlap`
  (params (OverlappedComponent :type "PrimitiveComponent Object Reference") (OtherActor :type "Actor Object Reference") (OtherComp :type "PrimitiveComponent Object Reference") (OtherBodyIndex :type Integer) (bFromSweep :type Boolean) (SweepResult :type "HitResult Structure (by ref)")))

(event `self.Headshot.OnComponentBeginOverlap`
  (params (OverlappedComponent :type "PrimitiveComponent Object Reference") (OtherActor :type "Actor Object Reference") (OtherComp :type "PrimitiveComponent Object Reference") (OtherBodyIndex :type Integer) (bFromSweep :type Boolean) (SweepResult :type "HitResult Structure (by ref)")))

(fn `Damaged`
  (params (Damege :type "Float (double-precision)"))
  (`GameplayStatics.ApplyDamage` self Damege))

(fn `UpdateWalkSpeed`
  (params (newWalkSpeed :type "Float (double-precision)"))
  (set `CharacterMovementComponent.MaxWalkSpeed` newWalkSpeed (`self.CharacterMovement`)))

(fn `UpdateWarning`
  (params (warningText :type "Text (by ref)"))
  (`TextRenderComponent.K2_SetText` (`self.Warning`) warningText))

(fn `UserConstructionScript`)