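; BP_MiniMap is an actor that creates the minimap widget and feeds it live player data.
; On BeginPlay it creates WBP_MiniMap, caches the BP_gameStateBase, and adds the widget to the viewport hidden.
; Each tick it writes the player's location and yaw into the MPC_Minimap material parameter collection.
; It also hides the widget while the game state's IsSQCplay flag is set and shows it otherwise.
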(event `self.ReceiveBeginPlay`
  (bind _returnvalue (`|CreateWidget` "/Game/KSW/MiniMap/WBP_MiniMap.WBP_MiniMap_C"))
  (bind _asbp_game_state_base (cast `/Game/KYJ/SQC_Timer_GameInstance/BP_gameStateBase` (`GameplayStatics.GetGameState`)))
  (`UserWidget.AddToViewport` _returnvalue 0)
  (`Widget.SetVisibility` _returnvalue "Hidden"))

(event `self.ReceiveTick`
  (params (DeltaSeconds :type "Float (single-precision)"))
  (bind _returnvalue (`GameplayStatics.GetPlayerCharacter` 0))
  (bind (_returnvalue_roll _returnvalue_pitch _returnvalue_yaw) (`KismetMathLibrary.BreakRotator` (`self.K2_GetActorRotation` _returnvalue)))
  (`KismetMaterialLibrary.SetVectorParameterValue` "/Game/KSW/MiniMap/MPC_Minimap.MPC_Minimap" "Player Location" (`KismetMathLibrary.Conv_VectorToLinearColor` (`self.K2_GetActorLocation` _returnvalue)))
  (`KismetMaterialLibrary.SetScalarParameterValue` "/Game/KSW/MiniMap/MPC_Minimap.MPC_Minimap" "Player Yaw" _returnvalue_yaw)
  (if (`/Game/KYJ/SQC_Timer_GameInstance/BP_gameStateBase.isSQCplay` (stale `self.ReceiveBeginPlay` _asbp_game_state_base))
    (`Widget.SetVisibility` (stale `self.ReceiveBeginPlay` _returnvalue) "Hidden")
    (else
      (`Widget.SetVisibility` (stale `self.ReceiveBeginPlay` _returnvalue) "Visible"))))

(fn `UserConstructionScript`)