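; Garage area-discovery trigger Blueprint that rewards the player with score the first time they enter its box.
; On box overlap by the third-person character, an AreaDiscovered flag gates a score update on BP_gameStateBase.
; It then creates an InteractMissionScore widget showing the "AREA DISCOVERED +20XP" message and sets the flag so the reward does not repeat.
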(event `self.Box.OnComponentBeginOverlap`
  (params (OverlappedComponent :type "PrimitiveComponent Object Reference") (OtherActor :type "Actor Object Reference") (OtherComp :type "PrimitiveComponent Object Reference") (OtherBodyIndex :type Integer) (bFromSweep :type Boolean) (SweepResult :type "HitResult Structure (by ref)"))
  (cast `/Game/ThirdPerson/Blueprints/BP_ThirdPersonCharacter` OtherActor)
  (if (not (`self.AreaDiscovered`))
    (bind _asbp_game_state_base (cast `/Game/KYJ/SQC_Timer_GameInstance/BP_gameStateBase` (`GameplayStatics.GetGameState`)))
    (`/Game/KYJ/SQC_Timer_GameInstance/BP_gameStateBase.UpdateScore` _asbp_game_state_base 20)
    (bind _returnvalue (`|CreateWidget` "/Game/BigTriplexHouseVilla/Widgets/missionAndXp/interactMissionScore.interactMissionScore_C"))
    (`TextBlock.SetText` (`/Game/BigTriplexHouseVilla/Widgets/missionAndXp/interactMissionScore.MissionSuccessTxt` _returnvalue) "AREA DISCOVERED     +20XP")
    (`UserWidget.AddToViewport` _returnvalue 0)
    (set `self.AreaDiscovered` true)))

(fn `UserConstructionScript`)