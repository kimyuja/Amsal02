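; Interactive fridge that opens and closes its doors when the player holds G nearby.
; A box overlap toggles input and a key prompt, while a hold component shows a progress widget until release.
; Timelines play or reverse to rotate the left and right doors and slide the big door.
; The left-door timeline switches the character to FocusCamera, and leaving the box restores FollowCamera.
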(event `self.BoxColl.OnComponentBeginOverlap`
  (params (OverlappedComponent :type "PrimitiveComponent Object Reference") (OtherActor :type "Actor Object Reference") (OtherComp :type "PrimitiveComponent Object Reference") (OtherBodyIndex :type Integer) (bFromSweep :type Boolean) (SweepResult :type "HitResult Structure (by ref)"))
  ;[1 1 1] 콜리전 안으로 들어가면 아이콘 보여줌 / 콜리전 벗어나면 아이콘 가림
  (`self.EnableInput` (`GameplayStatics.GetPlayerController` 0))
  (`SceneComponent.SetVisibility` (`self.PushKeyWidget`) true false))

(event `self.BoxColl.OnComponentEndOverlap`
  (params (OverlappedComponent :type "PrimitiveComponent Object Reference") (OtherActor :type "Actor Object Reference") (OtherComp :type "PrimitiveComponent Object Reference") (OtherBodyIndex :type Integer))
  ;[1 1 1] 콜리전 안으로 들어가면 아이콘 보여줌 / 콜리전 벗어나면 아이콘 가림
  (`self.DisableInput` (`GameplayStatics.GetPlayerController` 0))
  (`SceneComponent.SetVisibility` (`self.PushKeyWidget`) false false)
  (bind _asbp_third_person_character (cast `/Game/ThirdPerson/Blueprints/BP_ThirdPersonCharacter` (`GameplayStatics.GetPlayerCharacter` 0)))
  (`ActorComponent.SetActive` (`/Game/ThirdPerson/Blueprints/BP_ThirdPersonCharacter.FocusCamera` _asbp_third_person_character) false true)
  (`ActorComponent.SetActive` (`SecondProjectCharacter.FollowCamera` _asbp_third_person_character) true false))

(event `leftDoorOpenClose`
  ;[1 1 1] G키 1.5초 hold 시 냉장고 상호작용 + 키 누르면 hold 하라는 위젯 표시
  (if (< (stale _newtrack_0) 1.0) :!label _label
    (bind (_direction _newtrack_0) (`Timeline|Timeline_2` :!label _label_2)
      (:`Update`
        (`SceneComponent.K2_SetRelativeRotation` (`self.LeftDoor`) (`KismetMathLibrary.MakeRotator` 0.0 0.0 _newtrack_0) false false)
        (bind _asbp_third_person_character (cast `/Game/ThirdPerson/Blueprints/BP_ThirdPersonCharacter` (`GameplayStatics.GetPlayerCharacter` 0)))
        (`ActorComponent.SetActive` (`/Game/ThirdPerson/Blueprints/BP_ThirdPersonCharacter.FocusCamera` _asbp_third_person_character) true false)
        (`ActorComponent.SetActive` (`SecondProjectCharacter.FollowCamera` _asbp_third_person_character) false false)))
    (else
      (goto _label_2 :!via `Reverse`))))

(event `EnhancedInput|/Game/BigTriplexHouseVilla/Input/IA_G`
  (params (ActionValue :type Boolean) (ElapsedSeconds :type "Float (double-precision)") (TriggeredSeconds :type "Float (double-precision)") (InputAction :type "InputAction Object Reference" :default "/Game/BigTriplexHouseVilla/Input/IA_G.IA_G"))
  ;[1 1 1] G키 1.5초 hold 시 냉장고 상호작용 + 키 누르면 hold 하라는 위젯 표시
  (:`Triggered`
    (goto _label))
  (:`Started`
    (bind _returnvalue (`AddComponent|NODE_AddAC_holdComp-1` :`keyPressed` "G"))
    (set `self.roundprogressbar` _returnvalue))
  (:`Canceled`
    (`Widget.RemoveFromParent` (`/Game/BigTriplexHouseVilla/Widgets/interaction/AC_holdComp.holdKeyWidget` (`self.roundprogressbar`)) :!label _label_3)
    (set `self.roundprogressbar` null))
  (:`Completed`
    (goto _label_3)))

(event `EnhancedInput|/Game/BigTriplexHouseVilla/Input/IA_G`
  (params (ActionValue :type Boolean) (ElapsedSeconds :type "Float (double-precision)") (TriggeredSeconds :type "Float (double-precision)") (InputAction :type "InputAction Object Reference" :default "/Game/BigTriplexHouseVilla/Input/IA_G.IA_G"))
  ;[1 1 1] G키 1.5초 hold 시 냉장고 상호작용 + 키 누르면 hold 하라는 위젯 표시
  (:`Triggered`
    (if (> (stale _newtrack_0) -1.0)
      (bind (_direction _newtrack_0) (`Timeline|Timeline_3` :!label _label_4)
        (:`Update`
          (`SceneComponent.K2_SetRelativeRotation` (`self.RightDoor`) (`KismetMathLibrary.MakeRotator` 0.0 0.0 _newtrack_0) false false)))
      (else
        (goto _label_4 :!via `Reverse`)))))

(event `EnhancedInput|/Game/BigTriplexHouseVilla/Input/IA_G`
  (params (ActionValue :type Boolean) (ElapsedSeconds :type "Float (double-precision)") (TriggeredSeconds :type "Float (double-precision)") (InputAction :type "InputAction Object Reference" :default "/Game/BigTriplexHouseVilla/Input/IA_G.IA_G"))
  ;[1 1 1] G키 1.5초 hold 시 냉장고 상호작용 + 키 누르면 hold 하라는 위젯 표시
  (:`Triggered`
    (if (> 1.0 (stale _newtrack_0))
      (bind (_direction _newtrack_0) (`Timeline|Timeline_0` :!label _label_5)
        (:`Update`
          (`SceneComponent.K2_SetRelativeTransform` (`self.BigDoor`) (`KismetMathLibrary.MakeTransform` (`KismetMathLibrary.MakeVector` 0.0 _newtrack_0)) false false)))
      (else
        (goto _label_5 :!via `Reverse`)))))

(fn `UserConstructionScript`)