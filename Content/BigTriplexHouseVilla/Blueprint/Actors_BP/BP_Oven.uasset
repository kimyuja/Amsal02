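; BP_Oven is an interactive oven whose door opens or closes when the player holds G nearby.
; A box trigger enables or disables actor input and toggles the prompt icon on overlap begin and end.
; IA_G shows a hold-G widget on start, removing it on cancel or completion.
; When triggered (after a 1.5s hold, per comments), a timeline plays or reverses based on its value, driving door roll.
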(event `self.BoxColl.OnComponentBeginOverlap`
  (params (OverlappedComponent :type "PrimitiveComponent Object Reference") (OtherActor :type "Actor Object Reference") (OtherComp :type "PrimitiveComponent Object Reference") (OtherBodyIndex :type Integer) (bFromSweep :type Boolean) (SweepResult :type "HitResult Structure (by ref)"))
  ;[1 1 1] 트리거 안에 들어가면 아이콘 표시 / 트리거 벗어나면 아이콘 숨김
  (`self.EnableInput` (`GameplayStatics.GetPlayerController` 0))
  (`SceneComponent.ToggleVisibility` (`self.icon`) false :!label _label))

(event `self.BoxColl.OnComponentEndOverlap`
  (params (OverlappedComponent :type "PrimitiveComponent Object Reference") (OtherActor :type "Actor Object Reference") (OtherComp :type "PrimitiveComponent Object Reference") (OtherBodyIndex :type Integer))
  ;[1 1 1] 트리거 안에 들어가면 아이콘 표시 / 트리거 벗어나면 아이콘 숨김
  (`self.DisableInput` (`GameplayStatics.GetPlayerController` 0))
  (goto _label))

(event `EnhancedInput|/Game/BigTriplexHouseVilla/Input/IA_G`
  (params (ActionValue :type Boolean) (ElapsedSeconds :type "Float (double-precision)") (TriggeredSeconds :type "Float (double-precision)") (InputAction :type "InputAction Object Reference" :default "/Game/BigTriplexHouseVilla/Input/IA_G.IA_G"))
  ;[1 1 1] G 키로 위젯 띄우기 / 1.5초 hold시 상호작용
  (:`Triggered`
    (if (< (stale _newtrack_0) 1.0)
      (bind (_direction _newtrack_0) (`Timeline|Timeline_0` :!label _label_2)
        (:`Update`
          (`SceneComponent.K2_SetRelativeRotation` (`self.SM_OvenDoor`) (`KismetMathLibrary.MakeRotator` _newtrack_0) false false)))
      (else
        (goto _label_2 :!via `Reverse`))))
  (:`Started`
    (bind _returnvalue (`|CreateWidget` "/Game/BigTriplexHouseVilla/Widgets/BP_holdG.BP_holdG_C"))
    (bind _output_get (set `self.holdG` _returnvalue))
    (`UserWidget.AddToViewport` _output_get 0))
  (:`Canceled`
    (bind _holdg (`self.holdG` :!label _label_3)
      (:`then`
        (`Widget.RemoveFromParent` _holdg)
        (set `self.holdG` null))
      (:`else`)))
  (:`Completed`
    (goto _label_3)))

(fn `UserConstructionScript`)