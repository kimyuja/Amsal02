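; Interactive door Blueprint that swings open or closed for the player and for Enemy actors.
; When BP_ThirdPersonCharacter overlaps the box, input and the PushEWidget prompt are enabled until it leaves; Enemy actors toggle the door on both entering and leaving.
; Pressing E toggles the door's yaw timeline and a separate lock pitch timeline, choosing direction from each track's current value, with a delay before the lock reverses.
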(event `self.BoxColl.OnComponentBeginOverlap`
  (params (OverlappedComponent :type "PrimitiveComponent Object Reference") (OtherActor :type "Actor Object Reference") (OtherComp :type "PrimitiveComponent Object Reference") (OtherBodyIndex :type Integer) (bFromSweep :type Boolean) (SweepResult :type "HitResult Structure (by ref)"))
  (cast `Enemy` OtherActor
    (:`then`
      (if (< (stale _newtrack_0) 1.0) :!label _label
        (bind (_direction _newtrack_0) (`Timeline|Timeline_0` :!label _label_2)
          (:`Update`
            (`SceneComponent.K2_SetRelativeRotation` (`self.Door`) (`KismetMathLibrary.MakeRotator` 0.0 0.0 _newtrack_0) false false)))
        (else
          (goto _label_2 :!via `Reverse`))))
    (:`CastFailed`
      (cast `/Game/ThirdPerson/Blueprints/BP_ThirdPersonCharacter` OtherActor)
      (`self.EnableInput` (`GameplayStatics.GetPlayerController` 0))
      (`SceneComponent.SetVisibility` (`self.pushEWidget`) true false))))

(event `self.BoxColl.OnComponentEndOverlap`
  (params (OverlappedComponent :type "PrimitiveComponent Object Reference") (OtherActor :type "Actor Object Reference") (OtherComp :type "PrimitiveComponent Object Reference") (OtherBodyIndex :type Integer))
  (cast `Enemy` OtherActor
    (:`then`
      (goto _label))
    (:`CastFailed`
      (cast `/Game/ThirdPerson/Blueprints/BP_ThirdPersonCharacter` OtherActor)
      (`self.DisableInput` (`GameplayStatics.GetPlayerController` 0))
      (`SceneComponent.SetVisibility` (`self.pushEWidget`) false false))))

(event `Key|E`
  (params (Key :type "Key Structure"))
  (:`Pressed`
    (goto _label)))

(event `Key|E`
  (params (Key :type "Key Structure"))
  (:`Pressed`
    (if (< (stale _newtrack_0) 1.0)
      (bind (_direction _newtrack_0) (`Timeline|Timeline_1` :!label _label_3)
        (:`Update`
          (`SceneComponent.K2_SetRelativeRotation` (`self.Lock`) (`KismetMathLibrary.MakeRotator` 0.0 _newtrack_0) false false)))
      (else
        (`KismetSystemLibrary.Delay` 2.5)
        (goto _label_3 :!via `Reverse`)))))

(fn `UserConstructionScript`)