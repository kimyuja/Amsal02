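; Interactable attic ladder that folds down and back up on a held key press and rewards the player for discovering the area.
; Overlapping the box collision enables input and shows the prompt widget, and IA_G shows a hold-progress widget while held.
; Each trigger alternates two timelines forward or reversed to pitch the two ladder meshes.
; The first lowering adds score through BP_gameStateBase and displays an XP popup.
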(event `self.BoxColl.OnComponentBeginOverlap`
  (params (OverlappedComponent :type "PrimitiveComponent Object Reference") (OtherActor :type "Actor Object Reference") (OtherComp :type "PrimitiveComponent Object Reference") (OtherBodyIndex :type Integer) (bFromSweep :type Boolean) (SweepResult :type "HitResult Structure (by ref)"))
  ;[1 1 1] 콜리전 범위 내에 들어가면 E 키를 누르라는 아이콘 보여줌
  (`self.EnableInput` (`GameplayStatics.GetPlayerController` 0))
  (`SceneComponent.SetVisibility` (`self.Widget`) true false))

(event `self.BoxColl.OnComponentEndOverlap`
  (params (OverlappedComponent :type "PrimitiveComponent Object Reference") (OtherActor :type "Actor Object Reference") (OtherComp :type "PrimitiveComponent Object Reference") (OtherBodyIndex :type Integer))
  ;[1 1 1] 콜리전 범위 내에 들어가면 E 키를 누르라는 아이콘 보여줌
  (`self.DisableInput` (`GameplayStatics.GetPlayerController` 0))
  (`SceneComponent.SetVisibility` (`self.Widget`) false false))

(event `EnhancedInput|/Game/BigTriplexHouseVilla/Input/IA_G`
  (params (ActionValue :type Boolean) (ElapsedSeconds :type "Float (double-precision)") (TriggeredSeconds :type "Float (double-precision)") (InputAction :type "InputAction Object Reference" :default "/Game/BigTriplexHouseVilla/Input/IA_G.IA_G"))
  (:`Triggered`
    ;[1 1 1] 홀드성공하면 다락방 계단 내려온다
    (`/Engine/EditorBlueprintResources/StandardMacros.FlipFlop`
      (:`A`
        (`|ExecutionSequence`
          (:`then_0`
            (bind (_direction _newtrack_0) (`Timeline|Timeline_2` :!label _label)
              (:`Update`
                (`SceneComponent.K2_SetRelativeRotation` (`self.SM_AtticLatter_1`) (`KismetMathLibrary.MakeRotator` 0.0 _newtrack_0) false false)
                (`/Engine/EditorBlueprintResources/StandardMacros.DoOnce` false ; Area Discovered +20XP
                  (:`Completed`
                    (bind _asbp_game_state_base (cast `/Game/KYJ/SQC_Timer_GameInstance/BP_gameStateBase` (`GameplayStatics.GetGameState`)))
                    (`/Game/KYJ/SQC_Timer_GameInstance/BP_gameStateBase.UpdateScore` _asbp_game_state_base 20)
                    (bind _returnvalue (`|CreateWidget` "/Game/BigTriplexHouseVilla/Widgets/missionAndXp/interactMissionScore.interactMissionScore_C"))
                    (bind _output_get (set `self.getXP` _returnvalue))
                    (`TextBlock.SetText` (`/Game/BigTriplexHouseVilla/Widgets/missionAndXp/interactMissionScore.MissionSuccessTxt` _output_get) "AREA DISCOVERED     +20XP")
                    (`UserWidget.AddToViewport` (`self.getXP`) 0))))))
          (:`then_1`
            (bind (_direction_2 _newtrack_0_2) (`Timeline|Timeline_3` :!label _label_2)
              (:`Update`
                (`SceneComponent.K2_SetRelativeRotation` (`self.SM_AtticLatter_2`) (`KismetMathLibrary.MakeRotator` 0.0 _newtrack_0_2) false false))))))
      (:`B`
        (`|ExecutionSequence`
          (:`then_0`
            (goto _label :!via `ReverseFromEnd`))
          (:`then_1`
            (goto _label_2 :!via `ReverseFromEnd`))))))
  (:`Started`
    (bind _returnvalue_2 (`AddComponent|NODE_AddAC_holdComp-0` :`maxHoldTime` 2.0 :`keyPressed` "G"))
    (set `self.holdWidget` _returnvalue_2))
  (:`Canceled`
    (`Widget.RemoveFromParent` (`/Game/BigTriplexHouseVilla/Widgets/interaction/AC_holdComp.holdKeyWidget` (`self.holdWidget`)) :!label _label_3)
    (set `self.holdWidget` null))
  (:`Completed`
    (goto _label_3)))

(fn `UserConstructionScript`)