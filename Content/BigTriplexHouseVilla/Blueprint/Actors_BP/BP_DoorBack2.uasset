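; BP_DoorBack2 is an interactive double door that the player opens and closes with the E key.
; Overlapping BoxColl enables input and shows two push-E prompt widgets, and leaving it disables input and hides them.
; A FlipFlop alternates between playing and reversing two timelines, which drive the relative yaw of DoorR and DoorL.
; The overlap events do not check which actor entered or left.
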(event `self.BoxColl.OnComponentBeginOverlap`
  (params (OverlappedComponent :type "PrimitiveComponent Object Reference") (OtherActor :type "Actor Object Reference") (OtherComp :type "PrimitiveComponent Object Reference") (OtherBodyIndex :type Integer) (bFromSweep :type Boolean) (SweepResult :type "HitResult Structure (by ref)"))
  (`self.EnableInput` (`GameplayStatics.GetPlayerController` 0))
  (`SceneComponent.SetVisibility` (`self.pushEWidget`) true false)
  (`SceneComponent.SetVisibility` (`self.pushEWidget1`) true false))

(event `self.BoxColl.OnComponentEndOverlap`
  (params (OverlappedComponent :type "PrimitiveComponent Object Reference") (OtherActor :type "Actor Object Reference") (OtherComp :type "PrimitiveComponent Object Reference") (OtherBodyIndex :type Integer))
  (`self.DisableInput` (`GameplayStatics.GetPlayerController` 0))
  (`SceneComponent.SetVisibility` (`self.pushEWidget`) false false)
  (`SceneComponent.SetVisibility` (`self.pushEWidget1`) false false))

(event `Key|E`
  (params (Key :type "Key Structure"))
  (:`Pressed`
    (`/Engine/EditorBlueprintResources/StandardMacros.FlipFlop`
      (:`A`
        (`|ExecutionSequence`
          (:`then_0`
            (bind (_direction _newtrack_0) (`Timeline|Timeline_2` :!label _label)
              (:`Update`
                (`SceneComponent.K2_SetRelativeRotation` (`self.DoorR`) (`KismetMathLibrary.MakeRotator` 0.0 0.0 _newtrack_0) false false))))
          (:`then_1`
            (bind (_direction_2 _newtrack_0_2) (`Timeline|Timeline_1` :!label _label_2)
              (:`Update`
                (`SceneComponent.K2_SetRelativeRotation` (`self.DoorL`) (`KismetMathLibrary.MakeRotator` 0.0 0.0 _newtrack_0_2) false false))))))
      (:`B`
        (`|ExecutionSequence`
          (:`then_0`
            (goto _label :!via `ReverseFromEnd`))
          (:`then_1`
            (goto _label_2 :!via `ReverseFromEnd`)))))))

(fn `UserConstructionScript`)