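; Inventory component for BP_ThirdPersonCharacter that handles item pickup, XP scoring and a circular in-world inventory display.
; The F input sphere-traces from the follow camera for BP_itemPickUp actors, then uses display names to award score, show an XP popup and update per-type counts.
; New item types are added to ItemSlots, and each pickup respawns RotateInventoryBox actors in an evenly spaced ring attached to the InventoryPivot.
; Debug keys print inventory information.
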(event Custom|OnActorBeginOverlap_Event
  (params (OverlappedActor :type Actor%20Object%20Reference) (OtherActor :type Actor%20Object%20Reference)))

(event Custom|getPivot
  ;[0 0 0] 이거 안 쓸 듯
)

(event Input|EnhancedActionEvents|EnhancedInputActionIA_F
  (params (ActionValue :type Boolean) (ElapsedSeconds :type Float%20%28double-precision%29) (TriggeredSeconds :type Float%20%28double-precision%29) (InputAction :type Input%20Action%20Object%20Reference :default "/Game/BigTriplexHouseVilla/Input/IA_F.IA_F"))
  (bind _follow_camera (Variables|Default|GetFollow%20Camera))
  (bind _firstitemloc (Variables|Default|GetfirstItemLoc))
  (bind _gamestatebase (Variables|Default|GetgameStateBase))
  (bind _returnvalue (Transformation|GetWorldLocation _follow_camera))
  ;[1 1 1] 추적하고 픽업해
  (:Started
    (bind (_outhit _returnvalue_2) (Collision|SphereTraceForObjects _returnvalue (+ _returnvalue (* (Math|Vector|GetForwardVector (Transformation|GetWorldRotation _follow_camera)) 1e+03)) 2e+01 (Utilities|Array|MakeArray "ObjectTypeQuery2") false 0 "ForDuration"))
    (if _returnvalue_2
      (bind _asbp_item_pick_up (Utilities|Casting|CastToBP_itemPickUp (.HitActor (Collision|BreakHitResult _outhit))))
      (bind _output_get (Variables|Default|SetAs%20BP%20Item%20Pick%20Up _asbp_item_pick_up))
      ;;[1 1 1] 주운 아이템이 coin이라면 score+=5 , 독/화분이라면 score+=10
      (if (Utilities|Enum|Equal(Enum) (Utilities|GetDisplayName _output_get) "coin")
        (Development|PrintString "주운 아이템->코인")
        (Variables|/Game/KYJ/SQC_Timer_GameInstance/BP_gameStateBase.BP_gameStateBase_C|SetScore _gamestatebase (+ (Variables|/Game/KYJ/SQC_Timer_GameInstance/BP_gameStateBase.BP_gameStateBase_C|GetScore (Variables|Default|GetgameStateBase)) 5))
        ;[1 1 1] 미션 성공 +XP UI 띄우기
        (bind _returnvalue_3 (UserInterface|CreateWidget "/Game/BigTriplexHouseVilla/Widgets/missionAndXp/interactMissionScore.interactMissionScore_C"))
        (bind _output_get_2 (Variables|Default|SetgetXP _returnvalue_3))
        (Rendering|Components|TextRender|SetText (Variables|/Game/BigTriplexHouseVilla/Widgets/missionAndXp/interactMissionScore.interactMissionScore_C|GetMissionSuccessTxt _output_get_2) "COIN OBTAINED     +5XP")
        (UserInterface|Viewport|AddtoViewport (Variables|Default|GetgetXP) 0)
        ;[1 1 1] 주운 아이템별 개수 체크
        (Math|Integer|IncrementInt (Variables|quantity|GetcoinCount)
          (:%20%20
            (Variables|Quantity|SethaveCoin true)))
        (else
          (Development|PrintString "주운 아이템->코인X")
          (Variables|/Game/KYJ/SQC_Timer_GameInstance/BP_gameStateBase.BP_gameStateBase_C|SetScore _gamestatebase (+ (Variables|/Game/KYJ/SQC_Timer_GameInstance/BP_gameStateBase.BP_gameStateBase_C|GetScore (Variables|Default|GetgameStateBase)) 10))
          (bind _returnvalue_4 (UserInterface|CreateWidget "/Game/BigTriplexHouseVilla/Widgets/missionAndXp/interactMissionScore.interactMissionScore_C"))
          (bind _output_get_3 (Variables|Default|SetgetXP _returnvalue_4))
          (Rendering|Components|TextRender|SetText (Variables|/Game/BigTriplexHouseVilla/Widgets/missionAndXp/interactMissionScore.interactMissionScore_C|GetMissionSuccessTxt _output_get_3) "ITEM OBTAINED     +10XP")
          (UserInterface|Viewport|AddtoViewport (Variables|Default|GetgetXP) 0)
          (if (Utilities|Enum|Equal(Enum) (Utilities|GetDisplayName (Variables|Default|GetAs%20BP%20Item%20Pick%20Up)) "plant")
            (Math|Integer|IncrementInt (Variables|Quantity|GetplantCount)
              (:%20%20
                (Variables|Quantity|SethavePlant true)))
            (elif (Utilities|Enum|Equal(Enum) (Utilities|GetDisplayName (Variables|Default|GetAs%20BP%20Item%20Pick%20Up)) "poison")
              (Math|Integer|IncrementInt (Variables|Quantity|GetpoisonCount)
                (:%20%20
                  (Variables|Quantity|Sethavepoison true)))
              (elif (Utilities|Enum|Equal(Enum) (Utilities|GetDisplayName (Variables|Default|GetAs%20BP%20Item%20Pick%20Up)) "hammer")
                (Math|Integer|IncrementInt (Variables|Quantity|GethammerCount)
                  (:%20%20
                    (Variables|Quantity|SethaveHammer true)))
                (else
                  (Math|Integer|IncrementInt (Variables|Quantity|GetknifeCount)
                    (:%20%20
                      (Variables|Quantity|SethaveKnife true)))))))))
      ;[1 1 1] 이미 가지고 있는 아이템이니? 새로운 아이템이니?
      (for _array_element (Variables|Default|GetitemSlots)
        (if (== (.rowname (.item _array_element)) (Utilities|GetDisplayName _output_get))
          (Variables|Default|SetalreadyHaveItem true)))
      (if (Variables|Default|GetalreadyHaveItem)
        _
        (else
          ;[1 0.5516 0.5715] 새로운 아이템 -> 슬롯에 추가하고 월드에서 삭제
          ; 존재하는 아이템 -> 월드에서 삭제
          (CallFunction|AddItem (Variables|/Game/BigTriplexHouseVilla/Inventory/BP_itemPickUp.BP_itemPickUp_C|GetitemData _output_get))))
      (Actor|DestroyActor (Variables|Default|GetAs%20BP%20Item%20Pick%20Up))
      (Variables|Default|SetalreadyHaveItem false)
      (Development|PrintString (Utilities|String|Append "현재까지score : " (Utilities|String|ToString(Integer) (Variables|/Game/KYJ/SQC_Timer_GameInstance/BP_gameStateBase.BP_gameStateBase_C|GetScore (Variables|Default|GetgameStateBase)))))
      (if (Variables|Default|GetinventoryCreated)
        ;[1 1 1] 아이템 add 하고 바뀐 아이템 개수만큼 인벤토리 다시 구성해야 하는 경우  이전에 만든 인벤토리 박스들은 지움
        (for _index (range 0 (Variables|Default|GetitemCoount))
          (bind _returnvalue_5 (Actor|GetActorOfClass "/Game/BigTriplexHouseVilla/Inventory/rotateInventoryBox.rotateInventoryBox_C"))
          (bind _asrotate_inventory_box (Utilities|Casting|CastTorotateInventoryBox _returnvalue_5))
          (bind _output_get_4 (Variables|Default|SetAs%20Rotate%20Inventory%20Box _asrotate_inventory_box))
          (Actor|DestroyActor _output_get_4)))
      (Development|PrintString "아이템 획득!")
      (bind _output_get_5 (Variables|Default|SetitemCoount (Utilities|Array|Length (Variables|Default|GetitemSlots))))
      (Development|PrintString (Utilities|String|Append "현재 아이템 개수: " (Utilities|String|ToString(Integer) _output_get_5)) true true "(R=0.000000,G=0.660000,B=1.000000,A=1.000000)" 5.0)
      ;[1 1 1] [원점 기준 좌표 회전]
      ;
      ; 지정해 놓은 inventoryPivot의
      ; y축 기준 일정 거리(radius = y1) 떨어져
      ; x1 위치 기준 360/itemCount(degree)만큼씩 회전하며 액터(box staticmesh) 스폰
      (Variables|Default|Setdegree (Math|Conversions|ToFloat(Integer) (/ 360 (Variables|Default|GetitemCoount))))
      (for _index_2 (range 0 (- (Variables|Default|GetitemCoount) 1))
        (bind _returnvalue_6 (Game|SpawnActorfromClass "/Game/BigTriplexHouseVilla/Inventory/rotateInventoryBox.rotateInventoryBox_C" (Math|Transform|MakeTransform (+ (Variables|Default|GetpivotLoc) (Math|Vector|MakeVector (- (* (.x _firstitemloc) (Math|Trig|Cos(Degrees) (* _index_2 (Variables|Default|Getdegree)))) (* (.y _firstitemloc) (Math|Trig|Sin(Degrees) (* _index_2 (Variables|Default|Getdegree))))) (+ (* (.x _firstitemloc) (Math|Trig|Sin(Degrees) (* _index_2 (Variables|Default|Getdegree)))) (* (.y _firstitemloc) (Math|Trig|Cos(Degrees) (* _index_2 (Variables|Default|Getdegree))))) 0.0)) "0, 0, 0" "1.000000,1.000000,1.000000") "AlwaysSpawn" "MultiplyWithRoot" 0 0))
        (Transformation|SetActorRelativeRotation _returnvalue_6 "0.000000,0.000000,-12.000000") ; 카메라랑 정면이 되는 각도로 회전
        (bind _output_get_6 (Variables|Default|SetcreatedBoxs _returnvalue_6))
        (Utilities|Array|Add (Variables|Default|GetitemArr) _output_get_6)
        (Transformation|AttachComponentToComponent _output_get_6 (Variables|/Game/BigTriplexHouseVilla/Inventory/inventoryPivot.inventoryPivot_C|GetCylinder (Variables|Default|GetAs%20Inventory%20Pivot)) "None" "KeepWorld" "KeepWorld" "KeepWorld" true))
      (Utilities|Array|Add (Variables|Default|GetitemArr) (Variables|Default|GetcreatedBoxs))
      (Variables|Default|SetinventoryCreated true))))

(event EventBeginPlay
  (bind _asbp_third_person_character (Utilities|Casting|CastToBP_ThirdPersonCharacter (Components|GetOwner)))
  (Variables|Default|SetAs%20BP%20Third%20Person%20Character _asbp_third_person_character) ; poison 있으면 변수 true 해주려고
  ;[1 1 1] promote to variable
  (bind _output_get (Variables|Default|SetFollow%20Camera (Variables|/Script/SecondProject.SecondProjectCharacter|GetFollowCamera _asbp_third_person_character)))
  (Variables|Default|SetFocusCamera _output_get)
  ;[1 1 1] 인벤토리 생성할 위치 피봇
  (bind _returnvalue (Actor|GetActorOfClass "/Game/BigTriplexHouseVilla/Inventory/inventoryPivot.inventoryPivot_C"))
  (bind _asinventory_pivot (Utilities|Casting|CastToinventoryPivot _returnvalue))
  (Variables|Default|SetAs%20Inventory%20Pivot _asinventory_pivot)
  (Variables|Default|SetpivotLoc (Transformation|GetWorldLocation (Variables|/Game/BigTriplexHouseVilla/Inventory/inventoryPivot.inventoryPivot_C|GetCylinder _asinventory_pivot)))
  ;[1 1 1] score 연결
  (bind _returnvalue_2 (Actor|GetActorOfClass "/Game/KYJ/SQC_Timer_GameInstance/BP_gameStateBase.BP_gameStateBase_C"))
  (Variables|Default|SetgameStateBase _returnvalue_2))

(event EventTick
  (params (DeltaSeconds :type Float%20%28single-precision%29)))

(event Input|KeyboardEvents|DebugKeyM
  (params (Key :type Key%20Structure :default "None") (ActionValue :type Input%20Action%20Value%20Structure))
  (bind _itemslots (Variables|Default|GetitemSlots))
  ;[1 1 1] 디버그)) inventory list 출력
  (:Pressed
    (for _array_element _itemslots
      (Development|PrintString (Utilities|String|ToString(Name) "None") true true "(R=0.000000,G=0.660000,B=1.000000,A=1.000000)" 5.0))
    (Development|PrintString (Utilities|String|ToString(Integer) (Utilities|Array|Length _itemslots)))))

(event Input|KeyboardEvents|DebugKeyN
  (params (Key :type Key%20Structure :default "None") (ActionValue :type Input%20Action%20Value%20Structure))
  ;[1 1 1] 디버그)) 아이템 소유한 개수 출력
  (:Pressed
    (Utilities|FlowControl|Sequence
      (:then_0
        (Development|PrintString (Utilities|String|Append "coinCount: " (Utilities|String|ToString(Integer) (Variables|quantity|GetcoinCount))) true true "(R=1.000000,G=0.500000,B=0.500000,A=1.000000)"))
      (:then_1
        (Development|PrintString (Utilities|String|Append "poisonCount: " (Utilities|String|ToString(Integer) (Variables|Quantity|GetpoisonCount))) true true "(R=1.000000,G=0.502887,B=0.502887,A=1.000000)"))
      (:then_2
        (Development|PrintString (Utilities|String|Append "hammerCount: " (Utilities|String|ToString(Integer) (Variables|Quantity|GethammerCount))) true true "(R=1.000000,G=0.502887,B=0.502887,A=1.000000)"))
      (:then_3
        (Development|PrintString (Utilities|String|Append "knifeCount: " (Utilities|String|ToString(Integer) (Variables|Quantity|GetknifeCount))) true true "(R=1.000000,G=0.502887,B=0.502887,A=1.000000)"))
      (:then_4
        (Development|PrintString (Utilities|String|Append "plantCount: " (Utilities|String|ToString(Integer) (Variables|Quantity|GetplantCount))) true true "(R=1.000000,G=0.502887,B=0.502887,A=1.000000)")))))

(event Input|KeyboardEvents|DebugKeyL
  (params (Key :type Key%20Structure :default "None") (ActionValue :type Input%20Action%20Value%20Structure)))

(fn AddItem
  (params (NewItem :type S%20Slots%20Structure%20%28by%20ref%29))
  (Utilities|Array|Add (Variables|Default|GetitemSlots) NewItem))