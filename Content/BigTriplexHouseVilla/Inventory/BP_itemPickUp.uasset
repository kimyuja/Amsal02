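; BP_itemPickUp is an item pickup actor for the inventory that takes its static mesh from a data table row during construction.
; When the third-person character overlaps its box, it enables input and shows the PushF prompt, reversing both on exit.
; The F key only sets the PressedF flag.
; PlayAnimation and EndAnimation hide and restore the prompt, and AddItem appends to ItemSlots, with no callers in this file.
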(event `Key|F`
  (params (Key :type "Key Structure"))
  (:`Pressed`
    (set `self.pressedF` true))
  (:`Released`
    (set `self.pressedF` false)))

(event `self.Box.OnComponentBeginOverlap`
  (params (OverlappedComponent :type "PrimitiveComponent Object Reference") (OtherActor :type "Actor Object Reference") (OtherComp :type "PrimitiveComponent Object Reference") (OtherBodyIndex :type Integer) (bFromSweep :type Boolean) (SweepResult :type "HitResult Structure (by ref)"))
  (cast `/Game/ThirdPerson/Blueprints/BP_ThirdPersonCharacter` OtherActor)
  (`self.EnableInput` (`GameplayStatics.GetPlayerController` 0))
  (`SceneComponent.SetVisibility` (`self.pushF`) true false))

(event `self.Box.OnComponentEndOverlap`
  (params (OverlappedComponent :type "PrimitiveComponent Object Reference") (OtherActor :type "Actor Object Reference") (OtherComp :type "PrimitiveComponent Object Reference") (OtherBodyIndex :type Integer))
  (cast `/Game/ThirdPerson/Blueprints/BP_ThirdPersonCharacter` OtherActor)
  (`self.DisableInput` (`GameplayStatics.GetPlayerController` 0))
  (`SceneComponent.SetVisibility` (`self.pushF`) false false))

(event `PlayAnimation`
  ;[0.4895 0.9901 1] 이게 문젠가
  (`SceneComponent.SetVisibility` (`self.pushF`) false false))

(event `EndAnimation`
  ;[0.4895 0.9901 1] 이게 문젠가
  (`SceneComponent.SetVisibility` (`self.pushF`) true false))

(fn `addItem`
  (params (NewItem :type "/Game/BigTriplexHouseVilla/Inventory/S_Slots Structure"))
  (locals (itemSlots :type "Array of /Game/BigTriplexHouseVilla/Inventory/S_Slots Structure"))
  (`KismetArrayLibrary.Array_Add` (`local.itemSlots`) NewItem))

(fn `UserConstructionScript`
  (bind _itemdata (`self.itemData`))
  (bind _returnvalue (`|GetDataTableRow` (break `DataTableRowHandle` (break `/Game/BigTriplexHouseVilla/Inventory/S_Slots` _itemdata)) (`.RowName` (break `DataTableRowHandle` (break `/Game/BigTriplexHouseVilla/Inventory/S_Slots` _itemdata))))
    (:`then`
      (`StaticMeshComponent.SetStaticMesh` (`self.StaticMesh`) (`.StaticMesh_8_A58FA0BB45871B28C9F104BD9808BD2D` (break `/Game/BigTriplexHouseVilla/Inventory/S_AssassinationItem` _returnvalue))))))