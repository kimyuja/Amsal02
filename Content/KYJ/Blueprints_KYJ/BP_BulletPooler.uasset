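; Object pool actor for pistol bullets that avoids spawning them at fire time.
; On BeginPlay it pre-spawns MaxPoolSize BP_PistolBullet actors at the SpawnBox transform, hides their meshes and stores them in BulletArray.
; GetPooledBullet removes the first available bullet, stores it as PooledBullet and teleports it to the given transform.
; It neither unhides bullets nor returns them to the pool.
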(event `self.ReceiveBeginPlay`
  (`|ExecutionSequence`
    (:`then_0`
      (set `self.PoolTransform` (`SceneComponent.K2_GetComponentToWorld` (`self.spawn box`))) ; 스폰 위치
    )
    (:`then_1`
      (for _ (range (`self.MaxPoolSize`))
        (bind _returnvalue (`|SpawnActorFromClass` "/Game/1_PistolSystemEffects/BP_PistolBullet.BP_PistolBullet_C" (`self.PoolTransform`) "AlwaysSpawn" "MultiplyWithRoot" null null))
        (`SceneComponent.SetHiddenInGame` (`/Game/1_PistolSystemEffects/BP_PistolBullet.StaticMesh` _returnvalue) true true) ; 안 보이게
        (`KismetArrayLibrary.Array_Add` (`self.BulletArray`) _returnvalue)))))

(event `Get Pooled Bullet`
  (params (teleportTransform :type "Transform Structure"))
  (bind _bulletarray (`self.BulletArray`))
  (if (> (`KismetArrayLibrary.Array_Length` _bulletarray) 0)
    (set `self.Pooled Bullet` (`|GetArrayItem` _bulletarray)) ; 가져온 총알
    (`KismetArrayLibrary.Array_Remove` (`self.BulletArray`)) ; 가져올 수 있는 총알 배열에서 제거
    (`self.K2_TeleportTo` (`self.Pooled Bullet`) (.location teleportTransform) (.rotation teleportTransform))))

(fn `UserConstructionScript`)