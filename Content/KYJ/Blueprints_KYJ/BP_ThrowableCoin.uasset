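; Throwable coin actor that acts as a distraction for BP_HitManAI characters.
; When a hitman overlaps its box, it waits briefly, passes the coin's location to that AI and calls its CoinReaction.
; Tick, throttled by a Delay, checks the stored AI's distance to the coin, destroying the actor shortly after the AI gets close and otherwise printing the distance.
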(event `self.ReceiveTick`
  (params (DeltaSeconds :type "Float (single-precision)"))
  (`KismetSystemLibrary.Delay` 1.0)
  (bind _returnvalue (`KismetMathLibrary.Vector_Distance` (`self.K2_GetActorLocation` (stale `self.Box.OnComponentBeginOverlap` _asbp_hit_man_ai)) (`SceneComponent.K2_GetComponentLocation` (`self.Coin`))))
  (if (< _returnvalue 150.0)
    (`KismetSystemLibrary.Delay` 5.0)
    (`self.K2_DestroyActor`)
    (else
      (`KismetSystemLibrary.PrintString` (`KismetStringLibrary.Conv_DoubleToString` _returnvalue)))))

(event `self.Box.OnComponentBeginOverlap`
  (params (OverlappedComponent :type "PrimitiveComponent Object Reference") (OtherActor :type "Actor Object Reference") (OtherComp :type "PrimitiveComponent Object Reference") (OtherBodyIndex :type Integer) (bFromSweep :type Boolean) (SweepResult :type "HitResult Structure (by ref)"))
  (bind _coin (`self.Coin`))
  (bind _asbp_hit_man_ai (cast `/Game/KSW/AI3/BP_HitManAI` OtherActor))
  (`KismetSystemLibrary.Delay` 2.0)
  (set `HitManAI.coinLoc` (`SceneComponent.K2_GetComponentLocation` _coin) _asbp_hit_man_ai)
  (`HitManAI.CoinReaction` _asbp_hit_man_ai _coin))

(fn `UserConstructionScript`)