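; BP_ModelCar is a car Blueprint that drives its Model component toward the position of its Scene component.
; A level sequence is meant to call CanGoCar, which sets a flag that lets Tick run GoCar every frame.
; GoCar moves Model without sweep by a fraction of the remaining distance, scaled by Speed and delta time, so it eases in as it nears the target.
; The flag is never cleared here.
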(event `CanGoCar`
  ;[0 0 0] 시퀀스에서 이 함수 호출
  (set `self.bCanGo` true))

(event `self.ReceiveTick`
  (params (DeltaSeconds :type "Float (single-precision)"))
  (if (`self.bCanGo`)
    (`self.GoCar`)))

(event `GoCar`
  (`SceneComponent.K2_SetWorldLocation` (`self.model`) (+ (`SceneComponent.K2_GetComponentLocation` (`self.model`)) (* (- (`SceneComponent.K2_GetComponentLocation` (`self.Scene`)) (`SceneComponent.K2_GetComponentLocation` (`self.model`))) (* (`self.Speed`) (`GameplayStatics.GetWorldDeltaSeconds`)))) false false))

(fn `UserConstructionScript`)