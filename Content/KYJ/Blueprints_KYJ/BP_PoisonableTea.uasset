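; BP_PoisonableTea is a tea prop that the player character can poison when standing close to it.
; Its sphere overlap shows or hides a widget and toggles CanPoison on the first BP_ThirdPersonCharacter found at BeginPlay.
; The overlaps do not check which actor entered or left.
; A Poisoned event makes the particle system visible to show the poisoned state.
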(event `self.ReceiveBeginPlay`
  (bind _outactors (`GameplayStatics.GetAllActorsOfClass` "/Game/ThirdPerson/Blueprints/BP_ThirdPersonCharacter.BP_ThirdPersonCharacter_C"))
  (set `self.BP_ThirdPersonCharacter` (`|GetArrayItem` _outactors)))

(event `self.Sphere.OnComponentBeginOverlap`
  (params (OverlappedComponent :type "PrimitiveComponent Object Reference") (OtherActor :type "Actor Object Reference") (OtherComp :type "PrimitiveComponent Object Reference") (OtherBodyIndex :type Integer) (bFromSweep :type Boolean) (SweepResult :type "HitResult Structure (by ref)"))
  (`SceneComponent.SetVisibility` (`self.Widget`) true false)
  (set `/Game/ThirdPerson/Blueprints/BP_ThirdPersonCharacter.bCanPoison?` true (`self.BP_ThirdPersonCharacter`)) ; 가까이 와야 독 탈 수 있음
)

(event `self.Sphere.OnComponentEndOverlap`
  (params (OverlappedComponent :type "PrimitiveComponent Object Reference") (OtherActor :type "Actor Object Reference") (OtherComp :type "PrimitiveComponent Object Reference") (OtherBodyIndex :type Integer))
  (`SceneComponent.SetVisibility` (`self.Widget`) false false)
  (set `/Game/ThirdPerson/Blueprints/BP_ThirdPersonCharacter.bCanPoison?` false (`self.BP_ThirdPersonCharacter`)))

(event `Poisoned`
  (`SceneComponent.SetVisibility` (`self.ParticleSystem`) true false))

(fn `UserConstructionScript`)