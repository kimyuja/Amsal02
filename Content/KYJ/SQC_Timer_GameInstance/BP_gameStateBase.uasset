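; Game state for a Hitman-style mission that tracks elapsed time, score, success and kill-objective flags.
; BeginPlay checks the game instance's OpeningSQCfinish flag so Tick counts time only after the opening sequence has played.
; On success, Tick records the total time once and shows the results screen widget.
; Helper functions update score and poison/plant flags, and save or load this state through Hitman_gameInstance.
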(event `self.ReceiveBeginPlay`
  ;[1 1 1] 보류
  ;;[1 1 1] Game Data(SaveGameKYJ) Save/Load 하려고
  (bind _ashitman_game_instance (cast `/Game/KYJ/SQC_Timer_GameInstance/Hitman_gameInstance` (`GameplayStatics.GetGameInstance`))) ; 게임 인스턴스에서 Load Game Data, Save Game Data
  (bind _output_get (set `self.My Game Instance` _ashitman_game_instance))
  ;;[1 1 1] 시작하자마자 타이머가 돌지 않게 방지
  ;;;[1 1 1] 다시 시작할때 시퀀스를 재생했는지 체크
  (if (`/Game/KYJ/SQC_Timer_GameInstance/Hitman_gameInstance.openingSQCfinish` _output_get)
    (set `self.isSQCplay` false)
    (`self.TimerInit`)
    (else
      (set `self.isSQCplay` true))))

(event `TimerInit`
  ;[1 1 1] 보류
  ;;[1 1 1] 시퀀스 끝나면 타이머 실행해
  (if (`self.isSQCplay`)
    _))

(event `self.ReceiveTick`
  (params (DeltaSeconds :type "Float (single-precision)"))
  (if (not (`self.isSQCplay`))
    (bind _output_get (set `self.curTime` (+ (`self.curTime`) DeltaSeconds))) ; 나중에 미션 성공 시 최종 결과 때 받아와야 하는 변수임
    (if (`self.isSucceed`)
      ;[1 1 1] True일 때 미션 성공 UI Widget Create
      (`/Engine/EditorBlueprintResources/StandardMacros.DoOnce` false
        (:`Completed`
          (set `self.totalTimetoSuccess` _output_get)
          (bind _returnvalue (`|CreateWidget` "/Game/BigTriplexHouseVilla/Widgets/resultUI/WB_resultsScreen.WB_resultsScreen_C"))
          (`UserWidget.AddToViewport` _returnvalue 0))))))

(fn `LoadGameStateKYJ`
  (bind _gamestategamedatakyj (`/Game/KYJ/SQC_Timer_GameInstance/Hitman_gameInstance.GameStateLoadGameData` (`self.My Game Instance`)))
  (`|ExecutionSequence`
    (:`then_0`
      (set `self.curTime` (break `/Game/KYJ/SQC_Timer_GameInstance/GameStateGameDataKYJ` _gamestategamedatakyj)))
    (:`then_1`
      (set `self.isSucceed` (`.isSucceed_5_8BEE3BA8492D9457D98316BFCD9167E2` (break `/Game/KYJ/SQC_Timer_GameInstance/GameStateGameDataKYJ` _gamestategamedatakyj))))
    (:`then_2`
      (set `self.totalTimetoSuccess` (`.totalTimetoSuccess_20_81F84C8A4A251AF33188F7B6390D0DFC` (break `/Game/KYJ/SQC_Timer_GameInstance/GameStateGameDataKYJ` _gamestategamedatakyj))))
    (:`then_4`
      (set `self.isPoisonCompleted` (`.isPoisonCompleted_12_41A08B7443E3B00E184A18868BD6E61C` (break `/Game/KYJ/SQC_Timer_GameInstance/GameStateGameDataKYJ` _gamestategamedatakyj))))
    (:`then_5`
      (set `self.isPlantCompleted` (`.isPlantCompleted_14_EF556CFC41C5AA0E6341AF8380F2CF13` (break `/Game/KYJ/SQC_Timer_GameInstance/GameStateGameDataKYJ` _gamestategamedatakyj))))
    (:`then_6`
      (set `self.isTargetKillCompleted` (`.isTargetKillCompleted_16_908112034A998975CFB2B9A4F0E7D517` (break `/Game/KYJ/SQC_Timer_GameInstance/GameStateGameDataKYJ` _gamestategamedatakyj))))
    (:`then_7`
      (set `self.Score` (`.Score_19_100C79EF4DF0BFFB64236DBE872190BC` (break `/Game/KYJ/SQC_Timer_GameInstance/GameStateGameDataKYJ` _gamestategamedatakyj))))))

(fn `SaveGameStateKYJ`
  (`/Game/KYJ/SQC_Timer_GameInstance/Hitman_gameInstance.GameStateSaveGameData` (`self.My Game Instance`) (make `/Game/KYJ/SQC_Timer_GameInstance/GameStateGameDataKYJ` (`self.curTime`) (`self.isSucceed`) (`self.totalTimetoSuccess`) false (`self.isPoisonCompleted`) (`self.isPlantCompleted`) (`self.isTargetKillCompleted`) (`self.Score`))))

(fn `UpdateAccidentKillBool`
  (params (NewParam :type String))
  (if (`KismetStringLibrary.Contains` NewParam "poison")
    (set `self.isPoisonCompleted` true)
    (else
      (set `self.isPlantCompleted` true))))

(fn `UpdateScore`
  (params (ScoreUpdate :type Integer))
  (set `self.Score` (+ ScoreUpdate (`self.Score`))))

(fn `UserConstructionScript`)